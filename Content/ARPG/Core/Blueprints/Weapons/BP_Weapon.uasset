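; BP_Weapon is a weapon actor that relays hits on monsters to whoever owns it.
; When its Hitbox overlaps a BP_GenericMonster, it sends an ApplyAttackDamage message to the owner with the sweep result and itself as damage causer.
; Enable and disable functions toggle the hitbox's overlap events to control when hits register.
; It also reports an interactable type and supplies VFX asset, spawn location and scale.
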(event `self.Hitbox.OnComponentBeginOverlap`
  (params (OverlappedComponent :type "PrimitiveComponent Object Reference") (OtherActor :type "Actor Object Reference") (OtherComp :type "PrimitiveComponent Object Reference") (OtherBodyIndex :type Integer) (bFromSweep :type Boolean) (SweepResult :type "HitResult Structure (by ref)"))
  (cast `/Game/ARPG/Core/AI/BP_GenericMonster` OtherActor)
  (message `/Game/ARPG/Core/Interfaces/BPI_Combat.ApplyAttackDamage` (`self.GetOwner`) SweepResult self))

(fn `DisableHitEvents`
  (set `PrimitiveComponent.bGenerateOverlapEvents` false (`self.Hitbox`)))

(fn `EnableHitEvents`
  (set `PrimitiveComponent.bGenerateOverlapEvents` true (`self.Hitbox`)))

(fn `GetInteractableType`
  (returns (InteractableType :type "/Game/ARPG/Core/Enums/E_InteractableType Enum"))
  (return "NewEnumerator1"))

(fn `GetVFXInfo`
  (returns (VFX :type "ParticleSystem Object Reference") (SpawnLocation :type "Vector Structure") (Scale :type "Vector Structure"))
  (return (`self.VFX`) (`SceneComponent.K2_GetComponentLocation` (`self.VFX_SpawnLocation`)) (`self.VFX_Size`)))

(fn `UserConstructionScript`)