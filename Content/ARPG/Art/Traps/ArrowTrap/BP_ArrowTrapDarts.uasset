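; Projectile dart for the arrow trap that damages characters it hits.
; Each tick it moves along its forward vector by TravelSpeed with a swept location update, unscaled by delta time.
; A mesh overlap with a BP_GenericCharacter applies fixed point damage, passing the dart's location as the hit direction, then destroys the dart.
; A short lifespan set at BeginPlay cleans up darts that miss.
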(event `self.ReceiveBeginPlay`
  (`self.SetLifeSpan` 5.0))

(event `self.ReceiveTick`
  (params (DeltaSeconds :type "Float (single-precision)"))
  (`self.K2_SetActorLocation` self (+ (`self.K2_GetActorLocation` self) (* (`self.GetActorForwardVector` self) (`self.TravelSpeed`))) true false))

(event `self.StaticMeshComponent.OnComponentBeginOverlap`
  (params (OverlappedComponent :type "PrimitiveComponent Object Reference") (OtherActor :type "Actor Object Reference") (OtherComp :type "PrimitiveComponent Object Reference") (OtherBodyIndex :type Integer) (bFromSweep :type Boolean) (SweepResult :type "HitResult Structure (by ref)"))
  (bind _asbp_generic_character (cast `/Game/ARPG/Core/Character/BP_GenericCharacter` OtherActor))
  (`GameplayStatics.ApplyPointDamage` _asbp_generic_character 10.0 (`self.K2_GetActorLocation` self) SweepResult null self)
  (`self.K2_DestroyActor` self))

(fn `UserConstructionScript`)