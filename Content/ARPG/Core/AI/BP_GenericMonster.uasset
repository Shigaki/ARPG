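; BP_GenericMonster is an ARPG AI monster that handles dealing melee damage to the player and taking damage.
; Hit-check events toggle Hitbox overlaps, with a DoOnce limiting each window to one point-damage hit, valued from a combat action map.
; Incoming point damage passes through a defense reduction formula into AIStatsComponent health.
; Radial damage is empty, and the hit VFX call and knockback launch are disconnected.
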(fn `OnRep_AttackingType`)

(fn `UserConstructionScript`)