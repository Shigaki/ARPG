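; BP_DefaultPlayerController is a player controller that handles movement input for BP_BasePlayer characters.
; On BeginPlay it adds the default Enhanced Input mapping context, and on possession it caches the pawn as the player reference.
; IA_Move drives movement along fixed world axes, X input on world Y and Y input on world X, independent of actor facing.
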(event `self.ReceiveBeginPlay`
  (bind _returnvalue (pcsubsystem `EnhancedInputLocalPlayerSubsystem` self))
  (`/Engine/EditorBlueprintResources/StandardMacros.IsValid` _returnvalue
    (:`Is Valid`
      (`EnhancedInputSubsystemInterface.AddMappingContext` _returnvalue "/Game/CoopAdventure/Core/EnhancedInput/InputMappingContext/IMC_PlayerDefaultMapping.IMC_PlayerDefaultMapping" 0 (struct)))))

(event `self.ReceivePossess`
  (params (PossessedPawn :type "Pawn Object Reference"))
  (bind _asbp_base_player (cast `/Game/CoopAdventure/Core/Characters/BP_BasePlayer` PossessedPawn))
  (set `self.PCharacterRef` _asbp_base_player))

(event `EnhancedInput|/Game/CoopAdventure/Core/EnhancedInput/InputActions/IA_Move`
  (params (ActionValue :type "Vector2D Structure") (ElapsedSeconds :type "Float (double-precision)") (TriggeredSeconds :type "Float (double-precision)") (InputAction :type "InputAction Object Reference" :default "/Game/CoopAdventure/Core/EnhancedInput/InputActions/IA_Move.IA_Move"))
  (:`Triggered`
    (`Pawn.AddMovementInput` (`self.PCharacterRef`) (0.0 1.0 0.0) ActionValue_X false)
    (`Pawn.AddMovementInput` (`self.PCharacterRef`) (1.0 0.0 0.0) ActionValue_Y false)))

(fn `UserConstructionScript`)