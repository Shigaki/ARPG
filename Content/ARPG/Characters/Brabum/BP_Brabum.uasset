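; Brabum is the player character for a top-down ARPG, with diagonal-axis movement, charge-based dashing, cursor-aimed melee combos, damage and death.
; Light, heavy and dodge presses are stored in CombatComponent's input buffer, then gated on consumption by disabled-action sets driven by combat states.
; CombatComponent supplies attack montages, StatsComponent handles health, speed and dash charges, and a perk query can grant double dash.
; Weapon overlaps damage monsters; death fades out and reloads the map.
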(event `ConsumePotion`)

(event `Key|Three`
  (params (Key :type "Key Structure"))
  (:`Pressed`
    (`self.SlowMotionEvent` 0.12 0.48)))

(event `self.ReceiveBeginPlay`
  ;[0 0 1] BeginPlay
  (`ActorComponent.Activate` (`self.Camera1`) false)
  (`self.EnableAllInputActions`)
  (`/Game/ARPG/Core/ActorComponents/StatsComponent.InitializeStatsComponent` (`self.StatsComponent`))
  (`/Game/ARPG/Core/ActorComponents/CombatComponent.SetCombatAction` (`self.CombatComponent`) "NewEnumerator0")
  (`/Game/ARPG/Core/ActorComponents/CombatComponent.SetCombatState` (`self.CombatComponent`) "NewEnumerator7")
  (`/Game/ARPG/Core/ActorComponents/CombatComponent.SetGeneralCombatState` (`self.CombatComponent`) "NewEnumerator0")
  (add `AnimInstance.OnMontageBlendingOut` (`self.GetAnimInstance`) (`|CreateDelegate` :!event `OnMontageBlendOut`))
  (add `AnimInstance.OnAllMontageInstancesEnded` (`self.GetAnimInstance`) (`|CreateDelegate` :!event `OnMontageInstanceEnd`)))

(event `InputAxis|MoveRight`
  (params (AxisValue :type "Float (single-precision)"))
  ;[0 1 0] Input
  (if (not (or (`self.IsActionDisabled` "NewEnumerator57") (`self.bDisableAllActions`)))
    (`self.AddMovementInput` (1.0 1.0 0.0) AxisValue)
    (`self.SetLastFacingDirection`)))

(event `InputAxis|MoveForward`
  (params (AxisValue :type "Float (single-precision)"))
  ;[0 1 0] Input
  (if (not (or (`self.IsActionDisabled` "NewEnumerator57") (`self.bDisableAllActions`)))
    (`self.AddMovementInput` (1.0 -1.0 0.0) AxisValue)
    (`self.SetLastFacingDirection`)))

(event `InputAction|Dodge`
  (params (Key :type "Key Structure"))
  ;[0 1 0] Input
  (:`Pressed`
    (`/Game/ARPG/Core/ActorComponents/CombatComponent.StoreBufferKey` (`self.CombatComponent`) "NewEnumerator3")))

(event `Dodge`
  (bind _combatcomponent (`self.CombatComponent`))
  ;[0 1 0] Input
  (if (> (`/Game/ARPG/Core/ActorComponents/StatsComponent.CurrentDashCharges` (`self.StatsComponent`)) 0)
    (`/Game/ARPG/Core/ActorComponents/CombatComponent.SetCombatState` _combatcomponent "NewEnumerator19")
    (`/Game/ARPG/Core/ActorComponents/CombatComponent.SetCombatAction` _combatcomponent "NewEnumerator3")
    (`self.K2_SetActorRotation` (`self.GetRotationForAction`))
    (`/Game/ARPG/Core/ActorComponents/StatsComponent.SetAcceleration` (`self.StatsComponent`) true 25000.0)
    (`/Game/ARPG/Core/ActorComponents/StatsComponent.SetWalkSpeed` (`self.StatsComponent`) true 2000.0)
    (`/Game/ARPG/Core/ActorComponents/StatsComponent.ConsumeDodgeCharge` (`self.StatsComponent`))
    (`|PlayMontage` (`self.Mesh`) "/Game/ARPG/Characters/Lina/Animations/Montages/AM_Dash.AM_Dash"
      (:`OnCompleted`
        _)
      (:`OnBlendOut`
        _)
      (:`OnInterrupted`
        _))
    (`/Game/ARPG/Core/ActorComponents/StatsComponent.SetAcceleration` (`self.StatsComponent`) false 0.0)
    (`/Game/ARPG/Core/ActorComponents/StatsComponent.SetWalkSpeed` (`self.StatsComponent`) false 0.0)
    (`/Game/ARPG/Core/ActorComponents/CombatComponent.SetCombatState` (`self.CombatComponent`) "NewEnumerator7")))

(event `InputAction|LightAttack`
  (params (Key :type "Key Structure"))
  ;[1 0 0] Combat
  (:`Pressed`
    (if (`self.CanPerformInputAction?` "NewEnumerator43")
      (set `self.InputAction` "NewEnumerator43")
      (`/Game/ARPG/Core/ActorComponents/CombatComponent.StoreBufferKey` (`self.CombatComponent`) "NewEnumerator43"))))

(event `Attack`
  ;[1 0 0] Combat
  (`/Engine/EditorBlueprintResources/StandardMacros.DoOnce` false :!label _label
    (:`Completed`
      (`self.IsCombatStateEqual` "NewEnumerator19"
        (:`true`
          (`self.IsInputBufferOpen`
            (:`true`
              (`/Game/ARPG/Core/ActorComponents/CombatComponent.SetCombatAction` (`self.CombatComponent`) "NewEnumerator55")
              (`self.ContinueAttack`))))
        (:`false`
          (`self.IsInputActionEqual` "NewEnumerator43"
            (:`true`
              (`/Game/ARPG/Core/ActorComponents/CombatComponent.SetCombatAction` (`self.CombatComponent`) "NewEnumerator2")
              (`self.ContinueAttack`))
            (:`false`
              (`self.IsInputActionEqual` "NewEnumerator58"
                (:`true`
                  (`/Game/ARPG/Core/ActorComponents/CombatComponent.SetCombatAction` (`self.CombatComponent`) "NewEnumerator16")
                  (`self.ContinueAttack`))))))))))

(event `self.EnableAttack`
  ;[1 0 0] Combat
  (goto _label :!via `Reset`))

(event `ContinueAttack`
  (bind _combatcomponent (`self.CombatComponent`))
  ;[1 0 0] Combat
  (if (not (`|EnumEquality` (`/Game/ARPG/Core/ActorComponents/CombatComponent.CurrentCombatState` (`self.CombatComponent`)) "NewEnumerator8"))
    (bind _mouseworldlocation (`self.Get Mouse World Location`))
    (`self.K2_SetActorRotation` (`KismetMathLibrary.Conv_VectorToRotator` _mouseworldlocation)))
  (`/Game/ARPG/Core/ActorComponents/CombatComponent.SetCombatState` (`self.CombatComponent`) "NewEnumerator8")
  (bind (_animmontage _montageactionname _playrate _intimetostartmontageat) (`/Game/ARPG/Core/ActorComponents/CombatComponent.GetCombatActionMontage` _combatcomponent (`/Game/ARPG/Core/ActorComponents/CombatComponent.CurrentCombatAction` _combatcomponent) (`self.AttackCount`)))
  (`/Engine/EditorBlueprintResources/StandardMacros.IsValid` _animmontage
    (:`Is Valid`
      (`/Game/ARPG/Core/ActorComponents/CombatComponent.PlayHighPriorityMontage` (`self.CombatComponent`) _animmontage _playrate _intimetostartmontageat)
      (bind _result (`/Engine/EditorBlueprintResources/StandardMacros.IncrementInt` (`self.AttackCount`))
        (:`  `
          (if (> _result (`/Game/ARPG/Core/ActorComponents/CombatComponent.MontageLastIndex` (`self.CombatComponent`)))
            (set `self.AttackCount` 0)))))
    (:`Is Not Valid`
      (`self.ResetMeleeAttack`)
      (`self.ResetCombatStates`))))

(event `InputAction|HeavyAttack`
  (params (Key :type "Key Structure"))
  ;[1 0 0] Combat
  (:`Pressed`
    (if (`self.CanPerformInputAction?` "NewEnumerator58")
      (set `self.InputAction` "NewEnumerator58")
      (`/Game/ARPG/Core/ActorComponents/CombatComponent.StoreBufferKey` (`self.CombatComponent`) "NewEnumerator58"))))

(event `self.ResetAttackCombo`
  ;[1 0 0] Combat
  (set `self.NextLightAttack` "light01")
  (set `self.NextHeavyAttack` "heavy01"))

(event `self.SetNextAttackCombo`
  (params (NextLightAttack :type Name) (NextHeavyAttack :type Name))
  ;[1 0 0] Combat
  (set `self.NextLightAttack` NextLightAttack)
  (set `self.NextHeavyAttack` NextHeavyAttack))

(event `self.DisableInputAction`
  (params (InputActionToDisable :type "/Game/ARPG/Core/Enums/E_InputAction Enum" :default "NewEnumerator57"))
  ;[1 1 0] Character States
  (`BlueprintSetLibrary.Set_Add` (`self.DisabledInputActions`) InputActionToDisable))

(event `self.DisableAllActions`
  ;[1 1 0] Character States
  (set `self.bDisableAllActions` true))

(event `self.EnableAllActions`
  ;[1 1 0] Character States
  (set `self.bDisableAllActions` false))

(event `self.EnableInputAction`
  (params (InputActionToEnable :type "/Game/ARPG/Core/Enums/E_InputAction Enum" :default "NewEnumerator57"))
  ;[1 1 0] Character States
  (`BlueprintSetLibrary.Set_Remove` (`self.DisabledInputActions`) InputActionToEnable))

(event `self.CombatComponent.OnCombatActionChanged`
  (params (CombatAction :type "/Game/ARPG/Core/Enums/E_CombatAction Enum" :default "NewEnumerator0"))
  ;[1 1 0] Character States
  (switch `/Game/ARPG/Core/Enums/E_CombatAction` CombatAction
    (:`NewEnumerator0`
      (`/Game/ARPG/Core/ActorComponents/StatsComponent.SetWalkSpeed` (`self.StatsComponent`) false 0.0))
    (:`NewEnumerator22`
      (`/Game/ARPG/Core/ActorComponents/StatsComponent.SetWalkSpeed` (`self.StatsComponent`) true 300.0))))

(event `self.CombatComponent.OnGeneralStateChanged`
  (params (GeneralState :type "/Game/ARPG/Core/Enums/E_GeneralCombatState Enum" :default "NewEnumerator0"))
  ;[1 1 0] Character States
  (switch `/Game/ARPG/Core/Enums/E_GeneralCombatState` GeneralState
    (:`NewEnumerator3`
      (`KismetSystemLibrary.PrintString` "IM DEAD"))))

(event `self.CombatComponent.OnCombatStateChanged`
  (params (CombatState :type "/Game/ARPG/Core/Enums/E_CombatState Enum" :default "NewEnumerator7"))
  ;[1 1 0] Character States
  (switch `/Game/ARPG/Core/Enums/E_CombatState` CombatState
    (:`NewEnumerator7`
      (`BlueprintSetLibrary.Set_Clear` (`self.DisabledInputActions`) :!label _label_2))
    (:`NewEnumerator16`
      (goto _label_2))
    (:`NewEnumerator8`
      (`BlueprintSetLibrary.Set_AddItems` (`self.DisabledInputActions`) (`|MakeArray` "NewEnumerator57" "NewEnumerator3" :!type "/Game/ARPG/Core/Enums/E_InputAction Enum")))
    (:`NewEnumerator12`
      (`BlueprintSetLibrary.Set_AddItems` (`self.DisabledInputActions`) (`|MakeArray` "NewEnumerator57" "NewEnumerator3" :!type "/Game/ARPG/Core/Enums/E_InputAction Enum")))
    (:`NewEnumerator19`
      (`BlueprintSetLibrary.Set_AddItems` (`self.DisabledInputActions`) (`|MakeArray` "NewEnumerator57" "NewEnumerator3" "NewEnumerator43" "NewEnumerator58" "NewEnumerator60" "NewEnumerator22" :!type "/Game/ARPG/Core/Enums/E_InputAction Enum") :!label _label_3))
    (:`NewEnumerator29`
      (goto _label_3))
    (:`NewEnumerator24`
      (goto _label_3))
    (:`NewEnumerator28`
      (goto _label_3))))

(event `self.PlayCameraShake`
  (params (CameraShakeType :type "/Game/ARPG/Core/Enums/E_CameraShakeType Enum" :default "NewEnumerator0"))
  ;[0 1 1] Misc
  (`PlayerController.ClientStartCameraShake` :`self` (`GameplayStatics.GetPlayerController` 0) :`Shake` (select `/Game/ARPG/Core/Enums/E_CameraShakeType` CameraShakeType :`NewEnumerator4` "/Game/ARPG/Core/Camera/Effects/BP_SmallCameraShake.BP_SmallCameraShake_C" :`NewEnumerator5` "/Game/ARPG/Core/Camera/Effects/BP_NormalCameraShake.BP_NormalCameraShake_C" :`NewEnumerator6` "/Game/ARPG/Core/Camera/Effects/BP_BigCameraShake.BP_BigCameraShake_C" :`NewEnumerator1` "/Game/ARPG/Core/Camera/Effects/BP_RegularAttackCameraShake.BP_RegularAttackCameraShake_C" :`NewEnumerator2` "/Game/ARPG/Core/Camera/Effects/BP_BigCameraShake.BP_BigCameraShake_C" :`NewEnumerator3` "/Game/ARPG/Core/Camera/Effects/BP_RegularAttackCameraShake.BP_RegularAttackCameraShake_C" :!type "CameraShakeBase Class Reference")))

(event `SlowMotionEvent`
  (params (SlowMotionStrength :type "Float (double-precision)") (SlowMotionDuration :type "Float (double-precision)"))
  ;[0 1 1] Misc
  (`GameplayStatics.SetGlobalTimeDilation` SlowMotionStrength)
  (`KismetSystemLibrary.Delay` SlowMotionDuration)
  (`GameplayStatics.SetGlobalTimeDilation` 1.0))

(event `PerkUpdate_Dash`
  ;[1 0.3694 0.1989] Perks
  (bind _success (`/Game/ARPG/Core/ActorComponents/PerkComponent.QueryPerk` (`self.PerkComponent`) "double_dash"))
  (if _success
    (set `/Game/ARPG/Core/ActorComponents/StatsComponent.MaxDashCharges` 2 (`self.StatsComponent`))))

(event `self.OnInputBufferConsumed`
  (params (InputToBuffer :type "/Game/ARPG/Core/Enums/E_InputAction Enum" :default "NewEnumerator57"))
  ;[0 1 0] Input
  (if (`self.CanPerformInputAction?` InputToBuffer)
    (switch `/Game/ARPG/Core/Enums/E_InputAction` InputToBuffer
      (:`NewEnumerator3`
        (`self.Dodge`))
      (:`NewEnumerator43`
        (`self.Attack` :!label _label_4))
      (:`NewEnumerator58`
        (goto _label_4))
      (:`NewEnumerator22`
        (`self.ConsumePotion`)))))

(event `self.CombatComponent.OnInputBufferOpen`
  ;[0 1 0] Input
  (set `self.bInputBufferOpen` true)
  (`self.EnableAttack`))

(event `self.CombatComponent.OnInputBufferClose`
  ;[0 1 0] Input
  (set `/Game/ARPG/Core/ActorComponents/CombatComponent.StoredBufferKey` "NewEnumerator57" (`self.CombatComponent`))
  (set `self.bInputBufferOpen` false))

(event `self.EnableAllInputActions`
  ;[0 1 0] Input
  (set `self.bInputDisabled` false))

(event `self.DisableAllInputActions`
  ;[0 1 0] Input
  (set `self.bInputDisabled` true))

(event `Key|One`
  (params (Key :type "Key Structure"))
  ;[1 0 0] Combat
  (:`Pressed`
    (`GameplayStatics.ApplyDamage` self 20.0 null null "/Script/Engine.DamageType")))

(event `self.HitReactEvent`
  ;[1 0 0] Combat
  (`AnimInstance.Montage_Play` (`self.GetAnimInstance`) "/Game/ARPG/Characters/Lina/Animations/Montages/AM_Lina_Hit.AM_Lina_Hit" 1.5 "MontageLength" 0.0 true)
  (`/Game/ARPG/Core/ActorComponents/CombatComponent.SetCombatState` (`self.CombatComponent`) "NewEnumerator29"))

(event `self.ReceivePointDamage`
  (params (Damage :type "Float (single-precision)") (DamageType :type "DamageType Object Reference") (HitLocation :type "Vector Structure") (HitNormal :type "Vector Structure") (HitComponent :type "PrimitiveComponent Object Reference") (BoneName :type Name) (ShotFromDirection :type "Vector Structure") (InstigatedBy :type "Controller Object Reference") (DamageCauser :type "Actor Object Reference") (HitInfo :type "HitResult Structure (by ref)"))
  ;[1 0 0] Combat
  (`self.CustomDamage` Damage (`.ImpactPoint` (`GameplayStatics.BreakHitResult` HitInfo)) DamageCauser))

(event `self.ReceiveRadialDamage`
  (params (DamageReceived :type "Float (single-precision)") (DamageType :type "DamageType Object Reference") (Origin :type "Vector Structure") (HitInfo :type "HitResult Structure (by ref)") (InstigatedBy :type "Controller Object Reference") (DamageCauser :type "Actor Object Reference"))
  ;[1 0 0] Combat
  (`self.CustomDamage` DamageReceived (`.ImpactPoint` (`GameplayStatics.BreakHitResult` HitInfo)) DamageCauser))

(event `CustomDamage`
  (params (Damage :type "Float (double-precision)") (ImpactPoint :type "Vector Structure") (DamageCauser :type "Actor Object Reference"))
  ;[1 0 0] Combat
  (`self.IsDead`
    (:`false`
      (`/Game/ARPG/Core/ActorComponents/StatsComponent.DamageHealth` (`self.StatsComponent`) (`KismetMathLibrary.FTrunc` Damage))
      (`self.PlayCameraShake` "NewEnumerator5"))))

(event `self.ReceiveDestroyed`
  ;[0 1 1] Misc
  (`GameplayStatics.OpenLevel` "TopDownExampleMap"))

(event `self.DeathEvent`
  ;[1 0 0] Combat
  (`self.IsDead`
    (:`false`
      (`self.DisableAllInputActions`)
      (`CharacterMovementComponent.SetMovementMode` (`self.CharacterMovement`) "MOVE_None" 0)
      (set `/Game/ARPG/Core/ActorComponents/CombatComponent.bIsDead?` true (`self.CombatComponent`))
      (`/Game/ARPG/Core/ActorComponents/CombatComponent.SetGeneralCombatState` (`self.CombatComponent`) "NewEnumerator3")
      (bind _returnvalue (`AnimInstance.Montage_Play` (`self.GetAnimInstance`) "/Game/ARPG/Characters/Lina/Animations/Montages/AM_Lina_Death.AM_Lina_Death" 1.0 "MontageLength" 0.0 true))
      (`KismetSystemLibrary.Delay` (- _returnvalue 0.5))
      (set `SkeletalMeshComponent.bPauseAnims` true (`self.Mesh`))
      (`KismetSystemLibrary.Delay` 1.0)
      (`PlayerCameraManager.StartCameraFade` :`self` (`GameplayStatics.GetPlayerCameraManager` 0) :`ToAlpha` 1.0 :`Duration` 1.0 :`bHoldWhenFinished` true)
      (`KismetSystemLibrary.Delay` 3.0)
      (`self.K2_DestroyActor`))))

(event `EnableRagDoll`
  (bind _mesh (`self.Mesh`))
  (bind _pelvisbonename (`self.PelvisBoneName`))
  ;[1 0 0] Combat
  (`PrimitiveComponent.SetCollisionResponseToAllChannels` (`self.CapsuleComponent`) "ECR_Ignore")
  (set `SpringArmComponent.bDoCollisionTest` false (`self.SpringArm1`))
  (`SceneComponent.K2_AttachToComponent` (`self.SpringArm1`) (`self.Mesh`) _pelvisbonename "KeepWorld" "KeepWorld" "KeepWorld" true)
  (`CharacterMovementComponent.SetMovementMode` (`self.CharacterMovement`) "MOVE_None" 0)
  (`PrimitiveComponent.SetCollisionProfileName` _mesh "Ragdoll" true)
  (`SkeletalMeshComponent.SetAllBodiesBelowSimulatePhysics` _mesh _pelvisbonename true true)
  (`SkeletalMeshComponent.SetAllBodiesBelowPhysicsBlendWeight` _mesh _pelvisbonename 1.0 false true))

(event `CheckHitStart`
  ;[1 0 0] Combat
  (set `PrimitiveComponent.bGenerateOverlapEvents` true (`self.WeaponHitbox`)))

(event `CheckHitEnd`
  ;[1 0 0] Combat
  (set `PrimitiveComponent.bGenerateOverlapEvents` false (`self.WeaponHitbox`)))

(event `self.WeaponHitbox.OnComponentBeginOverlap`
  (params (OverlappedComponent :type "PrimitiveComponent Object Reference") (OtherActor :type "Actor Object Reference") (OtherComp :type "PrimitiveComponent Object Reference") (OtherBodyIndex :type Integer) (bFromSweep :type Boolean) (SweepResult :type "HitResult Structure (by ref)"))
  ;[1 0 0] Combat
  (bind _asbp_generic_monster (cast `/Game/ARPG/AI/BP_GenericMonster` OtherActor))
  (`GameplayStatics.ApplyPointDamage` _asbp_generic_monster 20.0 (`self.K2_GetActorLocation`) SweepResult null self)
  (`KismetSystemLibrary.PrintString` (`KismetStringLibrary.Concat_StrStr` "Dealt " "20" " damage to " (`KismetSystemLibrary.GetDisplayName` OtherActor))))

(fn `CanPerformInputAction?`
  (params (InputAction :type "/Game/ARPG/Core/Enums/E_InputAction Enum" :default "NewEnumerator0"))
  (returns (`CanPerformInput?` :type Boolean))
  ;[0 0.7656 1] Is character in the disabled state?
  (if (or (`self.IsGeneralCombatStateEqual` "NewEnumerator4") (`self.bDisableAllActions`) (`self.IsActionDisabled` InputAction))
    (`self.ResetCombatStates`)
    (return false)
    (else
      (return true))))

(fn `Get Mouse World Location`
  (returns (MouseWorldLocation :type "Vector Structure"))
  (bind (_returnvalue_x _returnvalue_y) (`KismetMathLibrary.BreakVector` (`self.K2_GetActorLocation`)))
  (bind _hitresult (`PlayerController.GetHitResultUnderCursorForObjects` (`GameplayStatics.GetPlayerController` 0) (`|MakeArray` "ObjectTypeQuery1" :!type "EObjectTypeQuery Enum") true))
  (return (`KismetMathLibrary.ClampVectorSize` (- (`KismetMathLibrary.MakeVector` (.x (`.Location` (`GameplayStatics.BreakHitResult` _hitresult))) (.y (`.Location` (`GameplayStatics.BreakHitResult` _hitresult)))) (`KismetMathLibrary.MakeVector` _returnvalue_x _returnvalue_y)) 0.0 1.0)))

(fn `OnMontageBlendOut`
  (params (Montage :type "AnimMontage Object Reference") (bInterrupted :type Boolean))
  (bind _statscomponent (`self.StatsComponent`))
  (`self.IsDead`
    (:`false`
      (if bInterrupted
        (`/Game/ARPG/Core/ActorComponents/StatsComponent.SetAcceleration` _statscomponent false 0.0)
        (`/Game/ARPG/Core/ActorComponents/StatsComponent.SetWalkSpeed` _statscomponent false 0.0)))))

(fn `OnMontageInstanceEnd`
  (bind _combatcomponent (`self.CombatComponent`))
  (`self.IsDead`
    (:`false`
      ;[0 0.7891 1] Reset character actions & states
      (`/Game/ARPG/Core/ActorComponents/CombatComponent.SetCombatAction` (`self.CombatComponent`) "NewEnumerator0")
      (`/Game/ARPG/Core/ActorComponents/CombatComponent.SetCombatState` (`self.CombatComponent`) "NewEnumerator7")
      (if (`/Game/ARPG/Core/ActorComponents/CombatComponent.bCombatState` (`self.CombatComponent`))
        (`/Game/ARPG/Core/ActorComponents/CombatComponent.SetGeneralCombatState` _combatcomponent "NewEnumerator0")
        (else
          (`/Game/ARPG/Core/ActorComponents/CombatComponent.SetGeneralCombatState` _combatcomponent "NewEnumerator0")))
      (`self.ResetMeleeAttack`))))

(fn `ResetCombatStates`
  (bind _combatcomponent (`self.CombatComponent`))
  ;[0.6406 1 0] If no montage is playing reset character states and re-enable attack in case it was disabled
  (if (`AnimInstance.IsAnyMontagePlaying` (`self.GetAnimInstance`))
    (return)
    (else
      (`/Game/ARPG/Core/ActorComponents/CombatComponent.SetGeneralCombatState` _combatcomponent "NewEnumerator0")
      (`/Game/ARPG/Core/ActorComponents/CombatComponent.SetCombatAction` _combatcomponent "NewEnumerator0")
      (`self.EnableAttack`)
      (`KismetSystemLibrary.PrintString` "reset combat state")
      (return))))

(fn `ResetMeleeAttack`
  (set `self.AttackCount` 0)
  (set `self.MeleeAttackLastIndex` 0)
  (`self.EnableAttack`)
  (`KismetSystemLibrary.PrintString` "reset melee"))

(fn `SetLastFacingDirection`
  (bind _returnvalue (`self.GetLastMovementInputVector`))
  (if (`KismetMathLibrary.NotEqualExactly_VectorVector` _returnvalue)
    (set `self.LastFacingDirection` _returnvalue)))

(fn `UpdateBlessings`)

(fn `UpdatePerks`
  (`self.PerkUpdate_Dash`))

(fn `UserConstructionScript`)