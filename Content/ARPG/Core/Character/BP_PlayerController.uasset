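; BP_PlayerController is the ARPG player controller that handles perk tree UI input and mouse cursor feedback.
; On BeginPlay it caches BP_DefaultGameMode, then uses that game mode's PerkTreeUI to toggle the perk tree on the TogglePerkTreeUI action, flipping game pause with it.
; Holding the left mouse button switches the cursor to a text edit beam, and releasing it restores the default.
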(event `self.ReceiveBeginPlay`
  (bind _asbp_default_game_mode (cast `/Game/ARPG/Core/GameModes/BP_DefaultGameMode` (`GameplayStatics.GetGameMode`)))
  (set `self.GameModeRef` _asbp_default_game_mode))

(event `InputAction|TogglePerkTreeUI` :paused true
  (params (Key :type "Key Structure"))
  (:`Pressed`
    (`/Game/ARPG/Core/UI/Perks/W_PerkTreeUI.TogglePerkUI` (`/Game/ARPG/Core/GameModes/BP_DefaultGameMode.PerkTreeUI` (`self.GameModeRef`)))
    (`GameplayStatics.SetGamePaused` (not (`GameplayStatics.IsGamePaused`)))))

(event `Key|LeftMouseButton` :consume false
  (params (Key :type "Key Structure"))
  (:`Pressed`
    (set `self.CurrentMouseCursor` "TextEditBeam"))
  (:`Released`
    (set `self.CurrentMouseCursor` "Default")))

(fn `UserConstructionScript`)