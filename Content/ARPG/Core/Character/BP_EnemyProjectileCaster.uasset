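; Enemy projectile caster character that automatically fires fireballs on a fixed repeating interval.
; BeginPlay starts a looping timer whose event spawns a scaled-down BP_Projectile_Fireball in front of the capsule, facing the capsule's direction.
; Spawning adjusts for collisions but always succeeds, and the graph has no targeting or player detection.
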(event `self.ReceiveBeginPlay`
  (`KismetSystemLibrary.K2_SetTimerDelegate` (delegate `SpawnProjectile`) 5.0 true))

(event `SpawnProjectile`
  (bind _capsulecomponent (`self.CapsuleComponent`))
  (`|SpawnActorFromClass` "/Game/ARPG/Core/Blueprints/Projectiles/BP_Projectile_Fireball.BP_Projectile_Fireball_C" (`KismetMathLibrary.MakeTransform` (+ (`SceneComponent.K2_GetComponentLocation` _capsulecomponent) (* (`SceneComponent.GetForwardVector` _capsulecomponent) 200.0)) (`SceneComponent.K2_GetComponentRotation` _capsulecomponent) (0.66 0.66 0.66)) "AdjustIfPossibleButAlwaysSpawn" "OverrideRootScale" null null))

(fn `UserConstructionScript`
  (`parent.UserConstructionScript`))