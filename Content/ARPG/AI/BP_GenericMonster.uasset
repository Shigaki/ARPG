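; BP_GenericMonster is an ARPG AI monster character that deals melee damage to the player and gets knocked back when hit.
; CheckHitStart and CheckHitEnd toggle hitbox overlaps, with a DoOnce limiting point damage to one player hit per window.
; Damage values come from MapCombatActions, keyed by the current CombatAction.
; Incoming point damage launches it away from the damage causer without reducing health here; radial damage is an empty stub.
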(fn `OnRep_AttackingType`)

(fn `UserConstructionScript`)