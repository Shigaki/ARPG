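; BP_ArrowTrapButton is a trigger button that fires nearby arrow trap pillars when the player overlaps its skeletal mesh.
; A DoOnce gate calls ActivateTrap, which plays the button montage and activates every BP_ArrowTrapPillar overlapping ActivationArea.
; The gate re-arms after a short delay once the montage completes, preventing retriggers in the meantime.
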(event `ActivateTrap`
  (`|PlayMontage` (`self.SkeletalMeshComponent`) "/Game/ARPG/Art/Traps/ArrowTrap/AM_ArrowTrapActivate.AM_ArrowTrapActivate"
    (:`then`
      (for _array_element (`PrimitiveComponent.GetOverlappingActors` (`self.ActivationArea`) "/Game/ARPG/Art/Traps/ArrowTrap/BP_ArrowTrapPillar.BP_ArrowTrapPillar_C")
        (bind _asbp_arrow_trap_pillar (cast `/Game/ARPG/Art/Traps/ArrowTrap/BP_ArrowTrapPillar` _array_element))
        (`/Game/ARPG/Art/Traps/ArrowTrap/BP_ArrowTrapPillar.ActivateTrap` _asbp_arrow_trap_pillar)))
    (:`OnCompleted`
      (`KismetSystemLibrary.Delay` 2.0)
      (goto _label :!via `Reset`))))

(event `self.SkeletalMeshComponent.OnComponentBeginOverlap`
  (params (OverlappedComponent :type "PrimitiveComponent Object Reference") (OtherActor :type "Actor Object Reference") (OtherComp :type "PrimitiveComponent Object Reference") (OtherBodyIndex :type Integer) (bFromSweep :type Boolean) (SweepResult :type "HitResult Structure (by ref)"))
  (cast `/Game/ARPG/Core/Character/BP_Player` OtherActor)
  (`/Engine/EditorBlueprintResources/StandardMacros.DoOnce` false :!label _label
    (:`Completed`
      (`self.ActivateTrap`)
      (`KismetSystemLibrary.PrintString` "TRAP"))))

(fn `UserConstructionScript`)