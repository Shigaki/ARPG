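; BP_SwitchDoor is a sliding door that can start locked and is unlocked by pressing its referenced switch.
; A switch-press binding clears the lock and turns the light green, while the Construction Script previews red or green from the lock state.
; A box overlap enables input for BP_Player, so E plays the sliding timeline when unlocked.
; Leaving the box disables input and reverses the timeline to close the door.
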(event `self.ReceiveBeginPlay`
  (add `/Game/ARPG/Blueprints/Doors/BP_Switch.SwitchPressed` (`self.SwitchRef`) (delegate `UnlockDoor`)))

(event `UnlockDoor`
  (params (Switch :type "/Game/ARPG/Blueprints/Doors/BP_Switch Object Reference"))
  (if (== Switch (`self.SwitchRef`))
    (set `self.bIsLocked` false)
    (`LightComponent.SetLightColor` (`self.LockLight`) (struct :`R` 0.078081 :`G` 0.666667 :`A` 1.0) true)))

(event `self.Box.OnComponentBeginOverlap`
  (params (OverlappedComponent :type "PrimitiveComponent Object Reference") (OtherActor :type "Actor Object Reference") (OtherComp :type "PrimitiveComponent Object Reference") (OtherBodyIndex :type Integer) (bFromSweep :type Boolean) (SweepResult :type "HitResult Structure (by ref)"))
  (cast `/Game/ARPG/Core/Character/BP_Player` OtherActor)
  (`self.EnableInput` (`GameplayStatics.GetPlayerController` 0)))

(event `self.Box.OnComponentEndOverlap`
  (params (OverlappedComponent :type "PrimitiveComponent Object Reference") (OtherActor :type "Actor Object Reference") (OtherComp :type "PrimitiveComponent Object Reference") (OtherBodyIndex :type Integer))
  (cast `/Game/ARPG/Core/Character/BP_Player` OtherActor)
  (`self.DisableInput` (`GameplayStatics.GetPlayerController` 0))
  (bind (_direction _doorsliding) (`Timeline|DoorAnimation` :!via `Reverse` :!label _label)
    (:`Update`
      (`SceneComponent.K2_SetRelativeLocation` (`self.DoorMesh`) _doorsliding false false))))

(event `Key|E`
  (params (Key :type "Key Structure"))
  (:`Pressed`
    (if (not (`self.bIsLocked`))
      (goto _label))))

(fn `UserConstructionScript`
  (if (`self.bIsLocked`)
    (`LightComponent.SetLightColor` (`self.LockLight`) (struct :`R` 0.734375 :`B` 0.008821 :`A` 1.0) true)
    (else
      (`LightComponent.SetLightColor` (`self.LockLight`) (struct :`R` 0.078081 :`G` 0.666667 :`A` 1.0) true))))