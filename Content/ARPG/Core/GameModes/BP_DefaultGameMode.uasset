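; BP_DefaultGameMode is the ARPG game mode that manages the perk tree and blessing UI screens.
; On BeginPlay it creates the perk tree widget and adds it to the viewport.
; CreateBlessingUI shows a new blessing widget and pauses the game, and DestroyBlessingUI removes that widget and unpauses.
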(event `self.ReceiveBeginPlay`
  (bind _returnvalue (`|CreateWidget` "/Game/ARPG/Core/UI/Perks/W_PerkTreeUI.W_PerkTreeUI_C"))
  (bind _output_get (set `self.PerkTreeUI` _returnvalue))
  (`UserWidget.AddToViewport` _output_get 0))

(event `/Game/ARPG/Core/Interfaces/BPI_Blessing.CreateBlessingUI`
  (bind _returnvalue (`|CreateWidget` "/Game/ARPG/Core/UI/Blessing/W_BlessingUI.W_BlessingUI_C"))
  (bind _output_get (set `self.BlessingUI` _returnvalue))
  (`UserWidget.AddToViewport` _output_get 0)
  (`GameplayStatics.SetGamePaused` true))

(event `/Game/ARPG/Core/Interfaces/BPI_Blessing.DestroyBlessingUI`
  (`Widget.RemoveFromParent` (`self.BlessingUI`))
  (`GameplayStatics.SetGamePaused` false))

(fn `UserConstructionScript`)