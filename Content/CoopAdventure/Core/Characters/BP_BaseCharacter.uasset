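; BP_BaseCharacter is a character Blueprint that provides damage math for outgoing and incoming hits.
; CalculateOutgoingDamage multiplies attack power by a base multiplier, then by CritRate on a weighted random crit.
; The returned Crit flag re-evaluates that random roll, so it can disagree with the damage applied.
; DamageReductionFormula scales incoming damage by 100 / (100 + Defense), giving diminishing returns on defense.
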(fn `CalculateOutgoingDamage`
  (params (AttackPower :type "Float (double-precision)") (BaseMultiplier :type "Float (double-precision)") (CritChance :type "Float (double-precision)") (CritRate :type "Float (double-precision)"))
  (returns (OutgoingDamage :type "Float (double-precision)") (`bCrit?` :type Boolean))
  (locals (FinalDamage :type "Float (double-precision)"))
  (bind _returnvalue (`KismetMathLibrary.RandomBoolWithWeight` CritChance))
  (set `local.FinalDamage` (* AttackPower BaseMultiplier))
  (if _returnvalue
    (return (* (`local.FinalDamage`) CritRate) _returnvalue)
    (else
      (return (`local.FinalDamage`) _returnvalue))))

(fn `DamageReductionFormula`
  (params (IncomingDamage :type "Float (double-precision)") (Defense :type "Float (double-precision)"))
  (returns (FinalDamage :type "Float (double-precision)"))
  (return (* IncomingDamage (/ 100.0 (+ 100.0 Defense)))))

(fn `UserConstructionScript`)