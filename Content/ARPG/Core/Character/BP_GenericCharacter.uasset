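; BP_GenericCharacter is a generic ARPG character Blueprint that provides combat damage math.
; CalculateOutgoingDamage scales attack power by a multiplier, then applies the CritRate multiplier on a weighted random roll against CritChance.
; DamageReductionFormula scales incoming damage by 100/(100+Defense), so added defense gives diminishing returns.
; The file shows no callers linking the two functions, and the construction script is empty.
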(fn `CalculateOutgoingDamage`
  (params (AttackPower :type "Float (double-precision)") (BaseMultiplier :type "Float (double-precision)") (CritChance :type "Float (double-precision)") (CritRate :type "Float (double-precision)"))
  (returns (OutgoingDamage :type "Float (double-precision)"))
  (locals (FinalDamage :type "Float (double-precision)"))
  (set `local.FinalDamage` (* AttackPower BaseMultiplier))
  (if (`KismetMathLibrary.RandomBoolWithWeight` CritChance)
    (return (* (`local.FinalDamage`) CritRate))
    (else
      (return (`local.FinalDamage`)))))

(fn `DamageReductionFormula`
  (params (IncomingDamage :type "Float (double-precision)") (Defense :type "Float (double-precision)"))
  (returns (FinalDamage :type "Float (double-precision)"))
  (return (* IncomingDamage (/ 100.0 (+ 100.0 Defense)))))

(fn `UserConstructionScript`)